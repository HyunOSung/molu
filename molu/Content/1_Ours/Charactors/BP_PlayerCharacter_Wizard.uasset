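; Player wizard character with Enhanced Input movement, mission-object interaction, HUD, regenerating HP, EXP leveling, and game pause at zero HP.
; Each tick, a camera line trace aims the BulletStart component at the target point.
; Left click plays a cooldown-scaled attack montage, while a separate Shot function spawns projectiles with optional homing pitch offset and multishot spray.
; Number keys are test toggles for homing, penetration, explosion and multishot.
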(event `self.ReceiveBeginPlay`
  (bind _returnvalue (pcsubsystem `EnhancedInputLocalPlayerSubsystem` (`GameplayStatics.GetPlayerController` 0)))
  (`/Engine/EditorBlueprintResources/StandardMacros.IsValid` _returnvalue
    (:`Is Valid`
      (`EnhancedInputSubsystemInterface.AddMappingContext` _returnvalue "/Game/1_Ours/Charactors/InputContext_Player.InputContext_Player" 0 (struct))
      ;[1 1 1] 발사 쿨타임 최초 설정
      (set `self.CoolReset` (`self.ShootCool`))
      ;[1 1 1] HUD 가동 시작
      (bind _returnvalue_2 (`|CreateWidget` "/Game/1_Ours/UI/WidgetBP_HUD.WidgetBP_HUD_C" (`GameplayStatics.GetPlayerController` 0)))
      (bind _output_get (set `self.Widget` _returnvalue_2))
      (`UserWidget.AddToViewport` _output_get 0)
      ;[1 1 1] HP UI 가동
      (set `self.Player_HP` (`self.Player_MaxHP`))
      (bind _aswidget_bp_player_hp (cast `/Game/1_Ours/UI/WidgetBP_PlayerHP` (`WidgetComponent.GetUserWidgetObject` (`self.HP_Widget`))))
      (bind _output_get_2 (set `self.HP_bar_UI` _aswidget_bp_player_hp))
      (set `/Game/1_Ours/UI/WidgetBP_PlayerHP.WG_HPPercent` (/ (`self.Player_HP`) (`self.Player_MaxHP`)) _output_get_2))))

(event `Key|One`
  (params (Key :type "Key Structure"))
  ;[1 1 1] 테스트용 유도 활성화 버튼
  (:`Pressed`
    (if (`self.HomingTrue`)
      (bind _output_get (set `self.HomingTrue` false))
      (`KismetSystemLibrary.PrintString` (`KismetStringLibrary.Conv_BoolToString` _output_get))
      (else
        (bind _output_get_2 (set `self.HomingTrue` true))
        (`KismetSystemLibrary.PrintString` (`KismetStringLibrary.Conv_BoolToString` _output_get_2))))))

(event `EnhancedInput|/Game/1_Ours/Charactors/Input_Jump`
  (params (ActionValue :type Boolean) (ElapsedSeconds :type "Float (double-precision)") (TriggeredSeconds :type "Float (double-precision)") (InputAction :type "InputAction Object Reference" :default "/Game/1_Ours/Charactors/Input_Jump.Input_Jump"))
  ;[1 1 1] 마우스-카메라 / 키보드-움직임
  (:`Started`
    (`self.Jump`))
  (:`Completed`
    (`self.StopJumping`)))

(event `Key|Two`
  (params (Key :type "Key Structure"))
  ;[1 1 1] 테스트용 관통 활성화 버튼
  (:`Pressed`
    (if (`self.PenetrateTrue`)
      (bind _output_get (set `self.PenetrateTrue` false))
      (`KismetSystemLibrary.PrintString` (`KismetStringLibrary.Conv_BoolToString` _output_get))
      (else
        (bind _output_get_2 (set `self.PenetrateTrue` true))
        (`KismetSystemLibrary.PrintString` (`KismetStringLibrary.Conv_BoolToString` _output_get_2))))))

(event `self.ReceiveAnyDamage`
  (params (Damage :type "Float (single-precision)") (DamageType :type "DamageType Object Reference") (InstigatedBy :type "Controller Object Reference") (DamageCauser :type "Actor Object Reference"))
  ;[1 1 1] 플레이어 HP
  (bind _output_get (set `self.Player_HP` (- (`self.Player_HP`) Damage)))
  (`KismetSystemLibrary.PrintString` (`KismetStringLibrary.Conv_DoubleToString` _output_get) false)
  (set `/Game/1_Ours/UI/WidgetBP_PlayerHP.WG_HPPercent` (/ _output_get (`self.Player_MaxHP`)) (`self.HP_bar_UI`))
  (if (<= _output_get 0.0)
    (`GameplayStatics.SetGamePaused` true)))

(event `EnhancedInput|/Game/1_Ours/Charactors/Input_Move`
  (params (ActionValue :type "Vector2D Structure") (ElapsedSeconds :type "Float (double-precision)") (TriggeredSeconds :type "Float (double-precision)") (InputAction :type "InputAction Object Reference" :default "/Game/1_Ours/Charactors/Input_Move.Input_Move"))
  (bind (_returnvalue_roll _returnvalue_pitch _returnvalue_yaw) (`KismetMathLibrary.BreakRotator` (`self.GetControlRotation`)))
  ;[1 1 1] 마우스-카메라 / 키보드-움직임
  (:`Triggered`
    (`self.AddMovementInput` (`KismetMathLibrary.GetRightVector` (`self.GetControlRotation`)) ActionValue_X)
    (`self.AddMovementInput` (`KismetMathLibrary.GetForwardVector` (`KismetMathLibrary.MakeRotator` _returnvalue_roll 0.0 _returnvalue_yaw)) ActionValue_Y)))

(event `Key|Three`
  (params (Key :type "Key Structure"))
  ;[1 1 1] 테스트용 폭발 활성화 버튼
  (:`Pressed`
    (if (`self.ExplosionTrue`)
      (bind _output_get (set `self.ExplosionTrue` false))
      (`KismetSystemLibrary.PrintString` (`KismetStringLibrary.Conv_BoolToString` _output_get))
      (else
        (bind _output_get_2 (set `self.ExplosionTrue` true))
        (`KismetSystemLibrary.PrintString` (`KismetStringLibrary.Conv_BoolToString` _output_get_2))))))

(event `EnhancedInput|/Game/1_Ours/Charactors/Input_Look`
  (params (ActionValue :type "Vector2D Structure") (ElapsedSeconds :type "Float (double-precision)") (TriggeredSeconds :type "Float (double-precision)") (InputAction :type "InputAction Object Reference" :default "/Game/1_Ours/Charactors/Input_Look.Input_Look"))
  ;[1 1 1] 마우스-카메라 / 키보드-움직임
  (:`Triggered`
    (`self.AddControllerYawInput` ActionValue_X)
    (`self.AddControllerPitchInput` ActionValue_Y)))

(event `InputAction|Interact`
  (params (Key :type "Key Structure"))
  ;[1 1 1] 인터랙션 코드
  (:`Pressed`
    (for _array_element (`self.GetOverlappingActors` "/Game/1_Ours/BluePrint/BP_MissionObject.BP_MissionObject_C")
      (if (`KismetSystemLibrary.DoesImplementInterface` _array_element "/Game/1_Ours/BluePrint/BP_Interaction.BP_Interaction_C")
        (message `/Game/1_Ours/BluePrint/BP_Interaction.Interact` _array_element)
        (break)))))

(event `Key|Four`
  (params (Key :type "Key Structure"))
  ;[1 1 1] 테스트용 산탄 활성화 버튼
  (:`Pressed`
    (if (`self.MultiShotTrue`)
      (bind _output_get (set `self.MultiShotTrue` false))
      (`KismetSystemLibrary.PrintString` (`KismetStringLibrary.Conv_BoolToString` _output_get))
      (else
        (bind _output_get_2 (set `self.MultiShotTrue` true))
        (`KismetSystemLibrary.PrintString` (`KismetStringLibrary.Conv_BoolToString` _output_get_2))))))

(event `Key|LeftMouseButton`
  (params (Key :type "Key Structure"))
  (bind _shootcool (`self.ShootCool`))
  ;[1 1 1] 탄 발사
  (:`Pressed`
    (if (<= (`self.ShootCool`) (`self.CoolReset`))
      (set `self.CoolReset` 0.0)
      (set `self.Shot Start` true)
      (`self.PlayAnimMontage` "/Game/1_Ours/Resources/3D/Anim/Attack01Anim_Montage.Attack01Anim_Montage" (/ (`self.BaseCool`) (`self.ShootCool`)))
      (`KismetSystemLibrary.Delay` _shootcool)
      (set `self.CoolReset` _shootcool)
      (set `self.Shot Start` false))))

(event `self.ReceiveTick`
  (params (DeltaSeconds :type "Float (single-precision)"))
  (bind _player_hp (`self.Player_HP`))
  (bind _target_verctor (`self.Target_Verctor`))
  (bind _camera (`self.Camera`))
  (bind _bullet_start (`self.Bullet Start`))
  (bind _player_maxhp (`self.Player_MaxHP`))
  (bind _returnvalue (`SceneComponent.K2_GetComponentLocation` _bullet_start))
  (bind _returnvalue_2 (`SceneComponent.K2_GetComponentLocation` _camera))
  (bind (_returnvalue_roll _returnvalue_pitch _returnvalue_yaw) (`KismetMathLibrary.BreakRotator` (`KismetMathLibrary.FindLookAtRotation` _returnvalue _target_verctor)))
  ;[1 1 1] 타겟 위치 인식 라인 트레이싱
  (`|ExecutionSequence`
    (:`then_0`
      ;[1 1 1] HP Gradual recovery
      (if (>= _player_hp _player_maxhp) :!label _label
        (set `self.Player_HP` _player_maxhp)
        (else
          (`KismetSystemLibrary.Delay` 1.0)
          (bind _output_get (set `self.Player_HP` (+ _player_hp (`self.Recovery_Gradual`))))
          (set `/Game/1_Ours/UI/WidgetBP_PlayerHP.WG_HPPercent` (/ _output_get (`self.Player_MaxHP`)) (`self.HP_bar_UI`))
          (goto _label))))
    (:`then_1`
      (bind (_outhit _returnvalue_3) (`KismetSystemLibrary.LineTraceSingleForObjects` _returnvalue_2 (+ _returnvalue_2 (* (`KismetMathLibrary.GetForwardVector` (`SceneComponent.K2_GetComponentRotation` _camera)) (`self.Line_Distance`))) (`|MakeArray` "ObjectTypeQuery2" "ObjectTypeQuery1" :!type "EObjectTypeQuery Enum")))
      (if _returnvalue_3
        (bind (_bblockinghit _binitialoverlap _time _distance _location _impactpoint _normal _impactnormal _physmat _hitactor _hitcomponent _hitbonename _bonename _hititem _elementindex _faceindex _tracestart _traceend) (`GameplayStatics.BreakHitResult` _outhit))
        (set `self.Target_Verctor` _location)
        (else
          (set `self.Target_Verctor` _traceend)))
      (`KismetSystemLibrary.PrintString` (`KismetStringLibrary.Conv_VectorToString` _target_verctor) false)
      (`SceneComponent.K2_SetWorldTransform` _bullet_start (`KismetMathLibrary.MakeTransform` _returnvalue (`KismetMathLibrary.MakeRotator` _returnvalue_roll _returnvalue_pitch _returnvalue_yaw) (`SceneComponent.K2_GetComponentScale` _bullet_start)) false false)
      (set `self.LookRotation` (`KismetMathLibrary.MakeRotator` _returnvalue_roll _returnvalue_pitch _returnvalue_yaw)))
    (:`then_2`
      (if (<= (`self.Player_HP`) 0.0)
        (`KismetSystemLibrary.Delay` 6.0)
        (`GameplayStatics.SetGamePaused` true)))))

(fn `Add_Exp`
  (params (NewParam :type Integer))
  (returns (Level :type Integer))
  (bind _output_get (set `self.EXP` (+ NewParam (`self.EXP`))))
  (if (>= _output_get (`self.EXP_Needed`))
    (`/Engine/EditorBlueprintResources/StandardMacros.IncrementInt` (`self.Lv`)
      (:`  `
        (set `self.EXP` (- (`self.EXP`) (`self.EXP_Needed`)))
        (set `self.EXP_Needed` (`KismetMathLibrary.Clamp` (`KismetMathLibrary.FTrunc` (* (`self.EXP_Needed`) 1.09)) 0 100))
        (`GameplayStatics.PlaySound2D` "/Engine/VREditor/Sounds/UI/Camera_Shutter.Camera_Shutter" 1.0 1.0 0.0 null null)
        (return (`self.Lv`))))
    (else
      (`GameplayStatics.PlaySound2D` "/Engine/VREditor/Sounds/UI/Click_on_Button.Click_on_Button" 1.0 1.0 0.0 null null))))

(fn `Immediate_Recovery_HP`
  (bind _player_maxhp (`self.Player_MaxHP`))
  (bind _returnvalue (+ (* _player_maxhp (/ (`self.Recovery_Immediate`) 100.0)) (`self.Player_HP`)))
  (if (>= _returnvalue _player_maxhp)
    (set `self.Player_HP` _player_maxhp)
    (else
      (set `self.Player_HP` _returnvalue))))

(fn `Shot`
  (bind _homingtrue (`self.HomingTrue`))
  (bind _multishottrue (`self.MultiShotTrue`))
  (bind (_lookrotation_roll _lookrotation_pitch _lookrotation_yaw) (`KismetMathLibrary.BreakRotator` (`self.LookRotation`)))
  (bind (_returnvalue_location _returnvalue_rotation) (`KismetMathLibrary.BreakTransform` (`SceneComponent.K2_GetComponentToWorld` (`self.Bullet Start`))))
  (bind (_shot_rotation_roll _shot_rotation_pitch _shot_rotation_yaw) (`KismetMathLibrary.BreakRotator` (`/Game/1_Ours/BluePrint/BFL_ProjectileSpray.GetSprayAngle` (`KismetMathLibrary.GetForwardVector` _returnvalue_rotation) (`self.Max Angle`))))
  (`|ExecutionSequence`
    (:`then_0`
      (if (and _homingtrue _multishottrue)
        (for _ (range (`self.Shot Amount`))
          (`|SpawnActorFromClass` "/Game/1_Ours/Bullet/BP_Projectile_base.BP_Projectile_base_C" (`KismetMathLibrary.MakeTransform` _returnvalue_location (`KismetMathLibrary.MakeRotator` _shot_rotation_roll (+ _shot_rotation_pitch 45.0) _shot_rotation_yaw)) "AlwaysSpawn" "MultiplyWithRoot" null null))
        (return)))
    (:`then_1`
      (if _homingtrue
        _
        (elif _multishottrue
          (for _ (range (`self.Shot Amount`))
            (`|SpawnActorFromClass` "/Game/1_Ours/Bullet/BP_Projectile_base.BP_Projectile_base_C" (`KismetMathLibrary.MakeTransform` _returnvalue_location (`KismetMathLibrary.MakeRotator` _shot_rotation_roll _shot_rotation_pitch _shot_rotation_yaw)) "AlwaysSpawn" "MultiplyWithRoot" null null))
          (return))))
    (:`then_2`
      (if _multishottrue
        _
        (elif _homingtrue
          (`|SpawnActorFromClass` "/Game/1_Ours/Bullet/BP_Projectile_base.BP_Projectile_base_C" (`KismetMathLibrary.MakeTransform` _returnvalue_location (`KismetMathLibrary.MakeRotator` _lookrotation_roll (+ _lookrotation_pitch 45.0) _lookrotation_yaw)) "AlwaysSpawn" "MultiplyWithRoot" null null)
          (return))))
    (:`then_3`
      (if (not (or (`self.HomingTrue`) (`self.MultiShotTrue`)))
        (`|SpawnActorFromClass` "/Game/1_Ours/Bullet/BP_Projectile_base.BP_Projectile_base_C" (`KismetMathLibrary.MakeTransform` _returnvalue_location (`KismetMathLibrary.MakeRotator` _lookrotation_roll _lookrotation_pitch _lookrotation_yaw)) "AlwaysSpawn" "MultiplyWithRoot" null null)
        (return)))))

(fn `Shot End`
  (set `self.Shot Start` false))

(fn `UserConstructionScript`)