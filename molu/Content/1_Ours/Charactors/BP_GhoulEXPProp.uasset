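; BP_GhoulEXPProp is an experience pickup that homes in on the player.
; Each Tick it prints its distance to the player pawn and, within a short radius, eases toward it with MoveComponentTo.
; On overlap with BP_ThirdPersonCharacter it calls AddEXP and destroys itself.
; If Lv then differs from NowLv, it opens WidgetBP_Upgrade, shows the cursor and pauses the game.
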(event `self.MainCollison.OnComponentBeginOverlap`
  (params (OverlappedComponent :type "PrimitiveComponent Object Reference") (OtherActor :type "Actor Object Reference") (OtherComp :type "PrimitiveComponent Object Reference") (OtherBodyIndex :type Integer) (bFromSweep :type Boolean) (SweepResult :type "HitResult Structure (by ref)"))
  (bind _returnvalue (`GameplayStatics.GetPlayerController` 0))
  (bind _output_get (set `self.Conntact` true))
  (if _output_get
    (bind _asbp_third_person_character (cast `/Game/ThirdPerson/Blueprints/BP_ThirdPersonCharacter` OtherActor))
    (`/Game/ThirdPerson/Blueprints/BP_ThirdPersonCharacter.Add_EXP` _asbp_third_person_character (`self.GiveEXP`))
    (`self.K2_DestroyActor`)
    (if (!= (`/Game/ThirdPerson/Blueprints/BP_ThirdPersonCharacter.Lv` _asbp_third_person_character) (`/Game/ThirdPerson/Blueprints/BP_ThirdPersonCharacter.NowLv` _asbp_third_person_character))
      (bind _returnvalue_2 (`|CreateWidget` "/Game/1_Ours/UI/WidgetBP_Upgrade.WidgetBP_Upgrade_C" (`GameplayStatics.GetPlayerController` 0)))
      (`/Game/1_Ours/UI/WidgetBP_Upgrade.Selecting` _returnvalue_2)
      (`UserWidget.AddToViewport` _returnvalue_2 0)
      (`WidgetBlueprintLibrary.SetInputMode_GameOnly` _returnvalue)
      (set `PlayerController.bShowMouseCursor` true _returnvalue)
      (`GameplayStatics.SetGamePaused` true))))

(event `self.MainCollison.OnComponentEndOverlap`
  (params (OverlappedComponent :type "PrimitiveComponent Object Reference") (OtherActor :type "Actor Object Reference") (OtherComp :type "PrimitiveComponent Object Reference") (OtherBodyIndex :type Integer))
  (set `self.Conntact` false))

(event `self.ReceiveTick`
  (params (DeltaSeconds :type "Float (single-precision)"))
  (bind _returnvalue (`SceneComponent.K2_GetComponentLocation` (`Actor.RootComponent` (`GameplayStatics.GetPlayerPawn` 0))))
  (bind _returnvalue_2 (`KismetMathLibrary.Vector_Distance` _returnvalue (`SceneComponent.K2_GetComponentLocation` (`self.DefaultSceneRoot`))))
  (`KismetSystemLibrary.PrintString` (`KismetStringLibrary.Conv_DoubleToString` _returnvalue_2))
  (if (<= _returnvalue_2 200.0)
    (`KismetSystemLibrary.MoveComponentTo` (`self.DefaultSceneRoot`) _returnvalue (struct) false false 0.5)))

(fn `UserConstructionScript`)