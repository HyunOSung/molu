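; BP_EXPProp is an experience pickup that drifts toward the player and grants EXP to the wizard character on overlap.
; Tick checks distance to the player pawn and, within a short radius, moves the root to its location with MoveComponentTo.
; Overlap adds the EXP and destroys the pickup; if the wizard's Lv and NowLv then differ, it opens the upgrade widget with current skill flags and pauses the game.
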(event `self.MainCollison.OnComponentBeginOverlap`
  (params (OverlappedComponent :type "PrimitiveComponent Object Reference") (OtherActor :type "Actor Object Reference") (OtherComp :type "PrimitiveComponent Object Reference") (OtherBodyIndex :type Integer) (bFromSweep :type Boolean) (SweepResult :type "HitResult Structure (by ref)"))
  (bind _output_get (set `self.Conntact` true))
  (if _output_get
    (bind _asbp_player_character_wizard (cast `/Game/1_Ours/Charactors/BP_PlayerCharacter_Wizard` OtherActor))
    (`/Game/1_Ours/Charactors/BP_PlayerCharacter_Wizard.Add_Exp` _asbp_player_character_wizard 0 (`self.GiveEXP`))
    (`self.K2_DestroyActor`)
    (if (!= (`/Game/1_Ours/Charactors/BP_PlayerCharacter_Wizard.Lv` _asbp_player_character_wizard) (`/Game/1_Ours/Charactors/BP_PlayerCharacter_Wizard.NowLv` _asbp_player_character_wizard))
      (bind _returnvalue (`|CreateWidget` "/Game/1_Ours/UI/WidgetBP_Upgrade.WidgetBP_Upgrade_C" (`GameplayStatics.GetPlayerController` 0)))
      (`/Game/1_Ours/UI/WidgetBP_Upgrade.Selecting` _returnvalue (`/Game/1_Ours/Charactors/BP_PlayerCharacter_Wizard.HomingTrue` _asbp_player_character_wizard) (`/Game/1_Ours/Charactors/BP_PlayerCharacter_Wizard.PenetrateTrue` _asbp_player_character_wizard) (`/Game/1_Ours/Charactors/BP_PlayerCharacter_Wizard.ExplosionTrue` _asbp_player_character_wizard) (`/Game/1_Ours/Charactors/BP_PlayerCharacter_Wizard.MultiShotTrue` _asbp_player_character_wizard))
      (`UserWidget.AddToViewport` _returnvalue 0)
      (`WidgetBlueprintLibrary.SetInputMode_GameOnly` (`GameplayStatics.GetPlayerController` 0))
      (`GameplayStatics.SetGamePaused` true))))

(event `self.MainCollison.OnComponentEndOverlap`
  (params (OverlappedComponent :type "PrimitiveComponent Object Reference") (OtherActor :type "Actor Object Reference") (OtherComp :type "PrimitiveComponent Object Reference") (OtherBodyIndex :type Integer))
  (set `self.Conntact` false))

(event `self.ReceiveTick`
  (params (DeltaSeconds :type "Float (single-precision)"))
  (bind _returnvalue (`SceneComponent.K2_GetComponentLocation` (`Actor.RootComponent` (`GameplayStatics.GetPlayerPawn` 0))))
  (if (<= (`KismetMathLibrary.Vector_Distance` _returnvalue (`SceneComponent.K2_GetComponentLocation` (`self.DefaultSceneRoot`))) 200.0)
    (`KismetSystemLibrary.MoveComponentTo` (`self.DefaultSceneRoot`) _returnvalue (struct) false false 0.5)))

(fn `UserConstructionScript`)