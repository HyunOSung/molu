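; BP_MissionObhectSpawner spawns BP_MissionObject actors at random reachable navmesh points, one after another as missions complete.
; BeginPlay waits, spawns the first object around the player pawn, then resets MissionCompleted and ObjectPos.
; Tick polls MissionCompleted, clears it, then after the same delay spawns another object within a wider radius of ObjectPos.
; Nothing in this graph sets MissionCompleted to true or updates ObjectPos to a real location.
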(event `self.ReceiveBeginPlay`
  (`KismetSystemLibrary.Delay` 30.0)
  (`|SpawnActorFromClass` "/Game/1_Ours/BluePrint/BP_MissionObject.BP_MissionObject_C" (`KismetMathLibrary.MakeTransform` (`NavigationSystemV1.K2_GetRandomReachablePointInRadius` (`self.K2_GetActorLocation` (`GameplayStatics.GetPlayerPawn` 0)) 3500.0 null null)) "Undefined" "MultiplyWithRoot" null null)
  (set `self.MissionCompleted` false)
  (set `self.ObjectPos` (0.0 0.0 0.0)))

(event `self.ReceiveTick`
  (params (DeltaSeconds :type "Float (single-precision)"))
  (if (`self.MissionCompleted`)
    (set `self.MissionCompleted` false)
    (`KismetSystemLibrary.Delay` 30.0)
    (`|SpawnActorFromClass` "/Game/1_Ours/BluePrint/BP_MissionObject.BP_MissionObject_C" (`KismetMathLibrary.MakeTransform` (`NavigationSystemV1.K2_GetRandomReachablePointInRadius` (`self.ObjectPos`) 5000.0 null null)) "Undefined" "MultiplyWithRoot" null null)))

(fn `UserConstructionScript`)