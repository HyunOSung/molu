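; Interactable mission objective that completes after the zone around it has been occupied long enough.
; A box shows the prompt to the player character; Interact starts the mission, swaps the cylinder material and reveals an enlarged sphere zone.
; While anything overlaps the sphere, a one-second Delay loop adds progress, which persists between overlaps.
; At maximum, Tick changes the material, waits, passes completion and position to the spawner, then destroys the actor.
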(event `self.ReceiveBeginPlay`
  (`SceneComponent.SetVisibility` (`self.Sphere`) false false))

(event `self.ReceiveTick`
  (params (DeltaSeconds :type "Float (single-precision)"))
  (bind _cylinder (`self.Cylinder`))
  (if (>= (`self.MissionProgress`) (`self.ProgressMax`))
    (`PrimitiveComponent.SetMaterial` _cylinder 0 "/Game/1_Ours/Material/MT_EndMission.MT_EndMission")
    (`KismetSystemLibrary.Delay` 5.0)
    (bind _returnvalue (`GameplayStatics.GetActorOfClass` "/Game/1_Ours/BluePrint/BP_MissionObhectSpawner.BP_MissionObhectSpawner_C"))
    (set `/Game/1_Ours/BluePrint/BP_MissionObhectSpawner.MissionCompleted` true _returnvalue)
    (set `/Game/1_Ours/BluePrint/BP_MissionObhectSpawner.ObjectPos` (`SceneComponent.K2_GetComponentLocation` _cylinder) _returnvalue)
    (`self.K2_DestroyActor`)))

(event `/Game/1_Ours/BluePrint/BP_Interaction.Interact`
  (bind _sphere (`self.Sphere`))
  (`PrimitiveComponent.SetMaterial` (`self.Cylinder`) 0 "/Game/1_Ours/Material/MT_OnMission.MT_OnMission")
  (`SceneComponent.SetHiddenInGame` (`self.Interaction Text`) true false)
  (`TextRenderComponent.K2_SetText` (`self.Interaction Text`) (`self.StartMission`))
  (`SceneComponent.SetVisibility` _sphere true false)
  (set `self.MissionStarted` true)
  (`SceneComponent.SetWorldScale3D` _sphere (35.0 35.0 35.0)))

(event `self.Box.OnComponentBeginOverlap`
  (params (OverlappedComponent :type "PrimitiveComponent Object Reference") (OtherActor :type "Actor Object Reference") (OtherComp :type "PrimitiveComponent Object Reference") (OtherBodyIndex :type Integer) (bFromSweep :type Boolean) (SweepResult :type "HitResult Structure (by ref)"))
  (cast `/Game/ThirdPerson/Blueprints/BP_ThirdPersonCharacter` OtherActor)
  (`SceneComponent.SetHiddenInGame` (`self.Interaction Text`) false false))

(event `self.Box.OnComponentEndOverlap`
  (params (OverlappedComponent :type "PrimitiveComponent Object Reference") (OtherActor :type "Actor Object Reference") (OtherComp :type "PrimitiveComponent Object Reference") (OtherBodyIndex :type Integer))
  (cast `/Game/ThirdPerson/Blueprints/BP_ThirdPersonCharacter` OtherActor)
  (`SceneComponent.SetHiddenInGame` (`self.Interaction Text`) true false))

(event `self.Sphere.OnComponentBeginOverlap`
  (params (OverlappedComponent :type "PrimitiveComponent Object Reference") (OtherActor :type "Actor Object Reference") (OtherComp :type "PrimitiveComponent Object Reference") (OtherBodyIndex :type Integer) (bFromSweep :type Boolean) (SweepResult :type "HitResult Structure (by ref)"))
  (bind _output_get (set `self.isOverlapped` true))
  (if (and _output_get (`self.MissionStarted`)) :!label _label
    (bind _output_get_2 (set `self.MissionProgress` (+ (`self.MissionProgress`) (`self.ProgressTick`))))
    (if (>= _output_get_2 (`self.ProgressMax`))
      (`KismetSystemLibrary.PrintString` "Activate Complete!")
      (else
        (`KismetSystemLibrary.PrintString` (`KismetStringLibrary.Conv_DoubleToString` _output_get_2))
        (`KismetSystemLibrary.Delay` 1.0)
        (goto _label)))))

(event `self.Sphere.OnComponentEndOverlap`
  (params (OverlappedComponent :type "PrimitiveComponent Object Reference") (OtherActor :type "Actor Object Reference") (OtherComp :type "PrimitiveComponent Object Reference") (OtherBodyIndex :type Integer))
  (set `self.isOverlapped` false))

(fn `UserConstructionScript`)