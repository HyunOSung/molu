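; Timed enemy spawner that places growing waves of weighted-random enemies around the player, in a ring whose outer radius widens over time.
; Each wave loads the five enemy-type weights from DT_Spawner by wizard player level, then picks classes by cumulative-sum roulette.
; Looping timers drive waves, radius growth and ChangeProbability, which shifts four weights toward limits, though the next successful table lookup overwrites them.
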(event `self.ReceiveBeginPlay`
  (`KismetSystemLibrary.K2_SetTimerDelegate` (delegate `RandomSpawner`) 10.0 true 10.0)
  (`KismetSystemLibrary.K2_SetTimerDelegate` (delegate `ExpandingSpawnArea`) 15.0 true 10.0)
  (`KismetSystemLibrary.K2_SetTimer` null "ChangeProbability" 60.0 true))

(event `RandomSpawner`
  (bind _returnvalue (`GameplayStatics.GetPlayerPawn` 0))
  (bind _spawnprobability (`self.SpawnProbability`))
  (bind (_returnvalue_roll _returnvalue_pitch) (`KismetMathLibrary.BreakRotator` (`self.K2_GetActorRotation` _returnvalue)))
  (for _ (range (+ (`self.SpawnNum`) 1))
    ;[1 1 1] 소환 확률 데이터 테이블
    (bind _asbp_player_character_wizard (cast `/Game/1_Ours/Charactors/BP_PlayerCharacter_Wizard` (`GameplayStatics.GetPlayerCharacter` 0)))
    (bind _returnvalue_2 (`|GetDataTableRow` "/Game/1_Ours/Data/DT_Spawner.DT_Spawner" (`KismetStringLibrary.Conv_StringToName` (`KismetStringLibrary.Conv_IntToString` (`/Game/1_Ours/Charactors/BP_PlayerCharacter_Wizard.Lv` _asbp_player_character_wizard))))
      (:`then`
        (`KismetArrayLibrary.Array_Set` _spawnprobability 0 (break `/Game/1_Ours/Data/STR_Spawn` _returnvalue_2))
        (`KismetArrayLibrary.Array_Set` _spawnprobability 1 (`.Ghoul_6_D8F658014D21772BF4F131B5F0BF4F7A` (break `/Game/1_Ours/Data/STR_Spawn` _returnvalue_2)))
        (`KismetArrayLibrary.Array_Set` _spawnprobability 2 (`.Skeleton_10_8E4731954AF2172FBABF47BDF2E24657` (break `/Game/1_Ours/Data/STR_Spawn` _returnvalue_2)))
        (`KismetArrayLibrary.Array_Set` _spawnprobability 3 (`.Ghoul_Enhanced_7_2374C2A148CF7FC5A5BF4BBB729B94BC` (break `/Game/1_Ours/Data/STR_Spawn` _returnvalue_2)))
        (`KismetArrayLibrary.Array_Set` _spawnprobability 4 (`.Lich_8_CC49ABA4433F911B1DA566BC1DA3AA7F` (break `/Game/1_Ours/Data/STR_Spawn` _returnvalue_2)))
        (bind _sumofval (`self.SumOfVal`))
        (bind _indexchosen (`self.DetremineIdex` (`KismetMathLibrary.RandomFloatInRange` 0.0 _sumofval)))
        (`|SpawnActorFromClass` (`|GetArrayItem` (`self.Enemy`) _indexchosen) (`KismetMathLibrary.MakeTransform` (+ (`self.K2_GetActorLocation` _returnvalue) (* (`KismetMathLibrary.Conv_RotatorToVector` (`KismetMathLibrary.MakeRotator` _returnvalue_roll _returnvalue_pitch (`KismetMathLibrary.RandomFloatInRange` 0.0 360.0))) (`KismetMathLibrary.RandomFloatInRange` 1000.0 (+ (`self.RangeWiderVar`) (`self.StartAreaVar`)))))) "Undefined" "MultiplyWithRoot" null null))))
  (set `self.SpawnNum` (+ (`self.SpawnNum`) 1)))

(event `ExpandingSpawnArea`
  (set `self.RangeWiderVar` (+ (`self.RangeWiderVar`) 125.0)))

(fn `ChangeProbability`
  (locals (MinusVar :type "Float (double-precision)" :default 5.0) (PlusVar :type "Float (double-precision)" :default 5.0) (MaxVal_0 :type "Float (double-precision)" :default 25.0) (MaxVal_1 :type "Float (double-precision)" :default 25.0) (MaxVal_2 :type "Float (double-precision)" :default 25.0) (MaxVal_3 :type "Float (double-precision)" :default 25.0))
  (bind _spawnprobability (`self.SpawnProbability`))
  (bind _maxval_3 (`local.MaxVal_3`))
  (bind _maxval_1 (`local.MaxVal_1`))
  (bind _maxval_2 (`local.MaxVal_2`))
  (bind _returnvalue (- (`|GetArrayItem` _spawnprobability 1) (`local.MinusVar`)))
  (bind _returnvalue_2 (- (`|GetArrayItem` _spawnprobability) (`local.MinusVar`)))
  (bind _returnvalue_3 (+ (`|GetArrayItem` _spawnprobability 3) (`local.PlusVar`)))
  (bind _returnvalue_4 (+ (`|GetArrayItem` _spawnprobability 2) (`local.PlusVar`)))
  (for _index (range (`KismetArrayLibrary.Array_Length` _spawnprobability))
    (switch `int` _index
      (:`0`
        (if (<= _returnvalue_2 (`local.MaxVal_0`))
          (`KismetArrayLibrary.Array_Set` _spawnprobability 0 (`local.MaxVal_0`))
          (else
            (`KismetArrayLibrary.Array_Set` _spawnprobability 0 _returnvalue_2))))
      (:`1`
        (if (<= _returnvalue _maxval_1)
          (`KismetArrayLibrary.Array_Set` _spawnprobability 1 _maxval_1)
          (else
            (`KismetArrayLibrary.Array_Set` _spawnprobability 1 _returnvalue))))
      (:`2`
        (if (<= _returnvalue_4 _maxval_2)
          (`KismetArrayLibrary.Array_Set` _spawnprobability 2 _returnvalue_4)
          (else
            (`KismetArrayLibrary.Array_Set` _spawnprobability 2 _maxval_2))))
      (:`3`
        (if (<= _returnvalue_3 _maxval_3)
          (`KismetArrayLibrary.Array_Set` _spawnprobability 3 _returnvalue_3)
          (else
            (`KismetArrayLibrary.Array_Set` _spawnprobability 3 _maxval_3))))))
  (return))

(fn `DetremineIdex`
  (params (RandomVal :type "Float (double-precision)"))
  (returns (IndexChosen :type Integer))
  (locals (LocalSum :type "Float (double-precision)"))
  (for (_array_element _array_index) (`self.SpawnProbability`)
    (bind _output_get (set `local.LocalSum` (+ _array_element (`local.LocalSum`))))
    (if (>= _output_get RandomVal)
      (break)))
  (return _array_index))

(fn `SumOfVal`
  (returns (SumofVal :type "Float (double-precision)"))
  (locals (LocalSum :type "Float (double-precision)"))
  (bind _localsum (`local.LocalSum`))
  (for _array_element (`self.SpawnProbability`)
    (set `local.LocalSum` (+ _array_element _localsum)))
  (return _localsum))

(fn `UserConstructionScript`)