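; Game manager actor that runs match flow for the wizard player: spawning, timer and level-up upgrades.
; BeginPlay waits briefly, moves the player to a random reachable navmesh point and starts background music.
; Once InGame is set, Tick spawns the enemy spawner once and starts a Delay loop counting seconds.
; Tick also watches for player level changes, opening the upgrade widget with UI-only input and pausing the game.
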(event `self.ReceiveBeginPlay`
  (bind _returnvalue (`GameplayStatics.GetPlayerCharacter` 0))
  (bind _randomlocation (`NavigationSystemV1.K2_GetRandomReachablePointInRadius` (`SceneComponent.K2_GetComponentLocation` (`self.DefaultSceneRoot`)) 5000.0 null null))
  (`self.K2_SetActorTransform` (`KismetMathLibrary.MakeTransform` (0.0 0.0 0.0)))
  (set `self.EnemySpawnerInGame` false)
  (bind _asbp_player_character_wizard (cast `/Game/1_Ours/Charactors/BP_PlayerCharacter_Wizard` _returnvalue))
  (set `self.P_Ref` _asbp_player_character_wizard)
  (`KismetSystemLibrary.Delay` 5.0)
  (`self.K2_SetActorLocation` _returnvalue (`KismetMathLibrary.MakeVector` (.x _randomlocation) (.y _randomlocation) (+ (.z _randomlocation) 100.0)) false false)
  (`GameplayStatics.SpawnSound2D` "/Game/1_Ours/Resources/Sound/BGM_2.BGM_2" 1.0 1.0 0.0 null))

(event `self.ReceiveTick`
  (params (DeltaSeconds :type "Float (single-precision)"))
  (bind _returnvalue (`GameplayStatics.GetPlayerController` 0))
  (bind _p_ref (`self.P_Ref`))
  (`|ExecutionSequence`
    (:`then_0`
      (if (`self.InGame`)
        (if (not (`self.EnemySpawnerInGame`))
          (`|SpawnActorFromClass` "/Game/1_Ours/BluePrint/BP_RandomSpawner.BP_RandomSpawner_C" (`SceneComponent.K2_GetComponentToWorld` (`self.DefaultSceneRoot`)) "Undefined" "MultiplyWithRoot" null null)
          (set `self.EnemySpawnerInGame` true)
          (`|ExecutionSequence`
            (:`then_0`
              (if (not (or (`GameplayStatics.IsGamePaused`) (`self.GameEnd`))) :!label _label
                (`/Engine/EditorBlueprintResources/StandardMacros.IncrementInt` (`self.TimePoint`)
                  (:`  `
                    (`KismetSystemLibrary.Delay` 1.0)
                    (goto _label)))))))))
    (:`then_1`
      (if (not (== (`/Game/1_Ours/Charactors/BP_PlayerCharacter_Wizard.Lv` _p_ref) (`/Game/1_Ours/Charactors/BP_PlayerCharacter_Wizard.NowLv` _p_ref)))
        (bind _returnvalue_2 (`|CreateWidget` "/Game/1_Ours/UI/WidgetBP_Upgrade.WidgetBP_Upgrade_C" _returnvalue))
        (`UserWidget.AddToViewport` _returnvalue_2 0)
        (`WidgetBlueprintLibrary.SetInputMode_UIOnlyEx` _returnvalue _returnvalue_2)
        (`GameplayStatics.SetGamePaused` true)))))

(fn `UserConstructionScript`)