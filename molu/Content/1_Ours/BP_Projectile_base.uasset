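; Base projectile Blueprint for a bullet that expires after a computed lifespan or destroys itself on hit.
; When ProjectileMovement activates, it applies BaseBulletSpeed as initial and max speed.
; It sets and debug-prints a lifespan of LineDistance / 10 divided by that speed.
; A comment says LineDistance matches Line_Distance in BP_ThirdPersonCharactor, with a data table planned later.
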(event `self.ProjectileMovement.OnComponentActivated`
  (params (Component :type "ActorComponent Object Reference") (bReset :type Boolean))
  (bind _projectilemovement (`self.ProjectileMovement`))
  (bind _base_bullet_speed (`self.Base_Bullet_Speed`))
  (bind _returnvalue (/ (/ (`self.Line_Distance`) 10.0) (`self.Base_Bullet_Speed`)))
  (set `ProjectileMovementComponent.InitialSpeed` _base_bullet_speed _projectilemovement)
  (set `ProjectileMovementComponent.MaxSpeed` _base_bullet_speed _projectilemovement)
  (`KismetSystemLibrary.PrintString` (`KismetStringLibrary.Conv_DoubleToString` _returnvalue))
  (`self.SetLifeSpan` _returnvalue))

(event `self.Base_bullet.OnComponentHit`
  (params (HitComponent :type "PrimitiveComponent Object Reference") (OtherActor :type "Actor Object Reference") (OtherComp :type "PrimitiveComponent Object Reference") (NormalImpulse :type "Vector Structure") (Hit :type "HitResult Structure (by ref)"))
  (`self.K2_DestroyActor`))

(fn `UserConstructionScript`)