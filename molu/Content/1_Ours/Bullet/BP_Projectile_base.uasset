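; Base projectile for the Wizard player, copying speed, range, damage, penetration and homing settings from the character when its movement component activates.
; Homing shots start under gravity, then repeatedly seek nearby "Enemy"-tagged actors via FindHomingTarget, while normal shots fly at bullet speed with a range-based lifespan.
; On overlap, the player's explosion and penetration flags select single-target or sphere-trace area damage and whether the projectile survives the hit.
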(event `self.ProjectileMovement.OnComponentActivated`
  (params (Component :type "ActorComponent Object Reference") (bReset :type Boolean))
  (bind _projectilemovement (`self.ProjectileMovement`))
  (bind _bullet_speed (`self.Bullet_Speed`))
  (bind _projectilemovement_2 (`self.ProjectileMovement`))
  ;[1 1 1] 최초 생성 설정
  (bind _asbp_player_character_wizard (cast `/Game/1_Ours/Charactors/BP_PlayerCharacter_Wizard` (`GameplayStatics.GetPlayerCharacter` 0)))
  (set `self.Bullet_Speed` (`/Game/1_Ours/Charactors/BP_PlayerCharacter_Wizard.BulletSpeed` _asbp_player_character_wizard))
  (set `self.Line_Distance` (`/Game/1_Ours/Charactors/BP_PlayerCharacter_Wizard.Line_Distance` _asbp_player_character_wizard))
  (set `self.Bullet_Damage` (`/Game/1_Ours/Charactors/BP_PlayerCharacter_Wizard.Damage` _asbp_player_character_wizard))
  (set `self.PenetrateCountLocal` (`/Game/1_Ours/Charactors/BP_PlayerCharacter_Wizard.PenetrateCount` _asbp_player_character_wizard))
  ;[1 1 1] 플레이어 유도가 트루일 경우 탄에 유도 속성 부여 후 유도 메커니즘 작동
  (if (`/Game/1_Ours/Charactors/BP_PlayerCharacter_Wizard.HomingTrue` _asbp_player_character_wizard)
    (`|ExecutionSequence`
      (:`then_0`
        (set `self.ProjectileHomingSpeed` (`/Game/1_Ours/Charactors/BP_PlayerCharacter_Wizard.HomingSpeed` _asbp_player_character_wizard)))
      (:`then_1`
        (set `ProjectileMovementComponent.ProjectileGravityScale` 1.0 _projectilemovement_2)
        (set `ProjectileMovementComponent.InitialSpeed` 1000.0 _projectilemovement_2)
        (`KismetSystemLibrary.Delay` 0.5)
        (set `ProjectileMovementComponent.ProjectileGravityScale` 0.0 _projectilemovement_2)
        (`self.FindHomingTarget` :!label _label)
        (`KismetSystemLibrary.Delay` 0.5)
        (goto _label))
      (:`then_2`
        (`self.SetLifeSpan` 1.5)))
    (else
      ;[1 1 1] 탄 이동 로직(일반)
      (set `ProjectileMovementComponent.InitialSpeed` _bullet_speed _projectilemovement)
      (set `ProjectileMovementComponent.MaxSpeed` _bullet_speed _projectilemovement)
      (`self.SetLifeSpan` (/ (- (`self.Line_Distance`) 400.0) (`self.Bullet_Speed`))))))

(event `self.Collison.OnComponentBeginOverlap`
  (params (OverlappedComponent :type "PrimitiveComponent Object Reference") (OtherActor :type "Actor Object Reference") (OtherComp :type "PrimitiveComponent Object Reference") (OtherBodyIndex :type Integer) (bFromSweep :type Boolean) (SweepResult :type "HitResult Structure (by ref)"))
  (bind _returnvalue (`SceneComponent.K2_GetComponentLocation` OverlappedComponent))
  (bind _bullet_damage (`self.Bullet_Damage`))
  (bind _returnvalue_2 (`self.K2_GetActorLocation` self))
  (bind _asbp_player_character_wizard (cast `/Game/1_Ours/Charactors/BP_PlayerCharacter_Wizard` (`GameplayStatics.GetPlayerCharacter` 0)))
  (`|ExecutionSequence`
    (:`then_0`
      ;[1 1 1] 폭발 관통 모두 True일 경우
      (if (and (`/Game/1_Ours/Charactors/BP_PlayerCharacter_Wizard.ExplosionTrue` _asbp_player_character_wizard) (`/Game/1_Ours/Charactors/BP_PlayerCharacter_Wizard.PenetrateTrue` _asbp_player_character_wizard))
        (bind _output_get (set `self.PenetrateCountLocal` (- (`self.PenetrateCountLocal`) 1)))
        (`KismetSystemLibrary.PrintString` (`KismetStringLibrary.Conv_IntToString` _output_get))
        (bind _outhits (`KismetSystemLibrary.SphereTraceMultiForObjects` _returnvalue_2 _returnvalue_2 (`/Game/1_Ours/Charactors/BP_PlayerCharacter_Wizard.ExplosionRadius` _asbp_player_character_wizard) (`self.Object Types`) false (`|MakeArray` self null :!type "Actor Object Reference") "ForDuration"))
        (for _array_element _outhits
          (`GameplayStatics.ApplyDamage` (`.HitActor` (`GameplayStatics.BreakHitResult` _array_element)) _bullet_damage)
          (if (not (> _output_get 0))
            (`self.K2_DestroyActor`)))))
    (:`then_1`
      ;[1 1 1] 관통만 True일 경우
      (if (`/Game/1_Ours/Charactors/BP_PlayerCharacter_Wizard.ExplosionTrue` _asbp_player_character_wizard)
        _
        (elif (`/Game/1_Ours/Charactors/BP_PlayerCharacter_Wizard.PenetrateTrue` _asbp_player_character_wizard)
          (bind _output_get_2 (set `self.PenetrateCountLocal` (- (`self.PenetrateCountLocal`) 1)))
          (`GameplayStatics.ApplyDamage` OtherActor _bullet_damage)
          (if (> _output_get_2 0)
            (`KismetSystemLibrary.PrintString` "Hello")
            (else
              (`KismetSystemLibrary.PrintString` "Hello2")
              (`self.K2_DestroyActor`))))))
    (:`then_2`
      ;[1 1 1] 폭발만 True일 경우
      (if (`/Game/1_Ours/Charactors/BP_PlayerCharacter_Wizard.PenetrateTrue` _asbp_player_character_wizard)
        _
        (elif (`/Game/1_Ours/Charactors/BP_PlayerCharacter_Wizard.ExplosionTrue` _asbp_player_character_wizard)
          (bind _outhits_2 (`KismetSystemLibrary.SphereTraceMultiForObjects` _returnvalue _returnvalue (`/Game/1_Ours/Charactors/BP_PlayerCharacter_Wizard.ExplosionRadius` _asbp_player_character_wizard) (`self.Object Types`) false (`|MakeArray` self null :!type "Actor Object Reference")))
          (for _array_element_2 _outhits_2
            (`GameplayStatics.ApplyDamage` (`.HitActor` (`GameplayStatics.BreakHitResult` _array_element_2)) _bullet_damage)
            (`self.K2_DestroyActor`)))))
    (:`then_3`
      ;[1 1 1] 일반 탄환(폭발 관통 모두 False)
      (if (not (or (`/Game/1_Ours/Charactors/BP_PlayerCharacter_Wizard.ExplosionTrue` _asbp_player_character_wizard) (`/Game/1_Ours/Charactors/BP_PlayerCharacter_Wizard.PenetrateTrue` _asbp_player_character_wizard)))
        (`GameplayStatics.ApplyDamage` OtherActor _bullet_damage)
        (`self.K2_DestroyActor`)))
    (:`then_4`
      (`/Engine/EditorBlueprintResources/StandardMacros.IsValid` "/Game/GreenwoodFantasyVillage/Blueprints/LandscapeModules/BP_Ground_16m_Hill.BP_Ground_16m_Hill"
        (:`Is Valid`
          (`KismetSystemLibrary.PrintString` "Hello")
          (`self.K2_DestroyActor`))))
    (:`then_5`
      (`/Engine/EditorBlueprintResources/StandardMacros.IsValid` "/Game/GreenwoodFantasyVillage/Blueprints/LandscapeModules/BP_Ground_16m.BP_Ground_16m"
        (:`Is Valid`
          (`KismetSystemLibrary.PrintString` "Hello")
          (`self.K2_DestroyActor`))))))

(fn `FindHomingTarget`
  (bind _projectilemovement (`self.ProjectileMovement`))
  (bind _outactors (`GameplayStatics.GetAllActorsOfClassWithTag` "/Script/Engine.Actor" "Enemy"))
  (for _array_element _outactors
    (bind _returnvalue (`KismetMathLibrary.VSize` (- (`self.K2_GetActorLocation` _array_element) (`self.K2_GetActorLocation`))))
    (if (< _returnvalue (`self.ClosestDistance`))
      (set `self.ClosestDistance` _returnvalue)
      (set `ProjectileMovementComponent.HomingTargetComponent` (`Actor.RootComponent` _array_element) _projectilemovement)
      (set `ProjectileMovementComponent.bIsHomingProjectile` true _projectilemovement)
      (set `ProjectileMovementComponent.HomingAccelerationMagnitude` (`self.ProjectileHomingSpeed`) _projectilemovement)
      (`self.K2_SetActorRotation` (`KismetMathLibrary.FindLookAtRotation` (`self.K2_GetActorLocation`) (`self.K2_GetActorLocation` _array_element)))))
  (return))

(fn `UserConstructionScript`)